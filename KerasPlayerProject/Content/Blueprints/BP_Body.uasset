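; Body actor that estimates a right and left joint position from two hand actors using a Keras neural network.
; BeginPlay loads the model from a project-relative file and builds an input tensor from both hands' relative locations and rotations.
; Each Tick refreshes the tensor, evaluates the model and converts its output to world-space joints using the actor transform.
; Debug lines and spheres show hand-joint-body chains, and a text component displays inference time.
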(event Custom|Draw_ConnectPoints
  (params (A :type Vector) (B :type Vector) (C :type Vector))
  ;[1 1 1] Helper Event to Draw
  (Rendering|Debug|DrawDebugLine A B "(R=1.000000,G=1.000000,B=1.000000,A=1.000000)" 0.0 1.0)
  (Rendering|Debug|DrawDebugLine B C "(R=1.000000,G=1.000000,B=1.000000,A=1.000000)" 0.0 1.0)
  (Rendering|Debug|DrawDebugSphere B 5.0 3 "(R=0.913311,G=0.419650,B=1.000000,A=1.000000)" 0.0 1.0))

(event EventBeginPlay
  (bind _returnvalue (Class|KismetSystemLibrary|GetProjectDirectory))
  (bind _modelpath (Variables|Default|GetModelPath))
  (bind _returnvalue_2 (Utilities|String|Append _returnvalue _modelpath))
  ;[1 1 1] Load Model from File
  (bind (_loadedmodel _returnvalue_3) (Class|KerasFunctionLibrary|CreateKerasModelfromFile (Game|GetGameMode) _returnvalue_2))
  (Variables|Default|SetKerasModel _loadedmodel)
  (if (Math|Boolean|ANDBoolean _returnvalue_3 (Utilities|IsValid (Variables|Default|GetHandRightActor)) (Utilities|IsValid (Variables|Default|GetHandLeftActor)))
    ;[1 1 1] Create input tensor
    (bind _returnvalue_4 (Class|KerasFunctionLibrary|CreateTensorfromArray (CallFunction|BuildInputData)))
    (Variables|Default|SetInputTensor _returnvalue_4)
    (else
      ;[1 1 1] Error Message
      (Development|PrintText (Utilities|Text|FormatText "Couldn't load Keras model file: {name}" _returnvalue_2) true true "(R=1.000000,G=0.140199,B=0.413809,A=1.000000)" 1e+01))))

(event EventTick
  (params (DeltaSeconds :type Float%20%28single-precision%29))
  (bind _returnvalue (Transformation|GetActorLocation))
  (if (Class|KerasModel|IsLoaded (Variables|Default|GetKerasModel))
    ;[1 1 1] Evaluate
    (Class|KerasFunctionLibrary|UpdateTensorfromArray (Variables|Default|GetInputTensor) (CallFunction|BuildInputData))
    (bind _outputdata (Class|KerasModel|Evaluate (Variables|Default|GetKerasModel) (Variables|Default|GetInputTensor)))
    ;[1 1 1] Draw Result
    (CallFunction|DrawConnectPoints (Transformation|GetActorLocation (Variables|Default|GetHandRightActor)) (.RightJoint (CallFunction|UnpackOutput (Class|KerasFunctionLibrary|TensorasFlatArray _outputdata))) _returnvalue)
    (CallFunction|DrawConnectPoints (Transformation|GetActorLocation (Variables|Default|GetHandLeftActor)) (.LeftJoint (CallFunction|UnpackOutput (Class|KerasFunctionLibrary|TensorasFlatArray _outputdata))) _returnvalue)
    ;[1 1 1] Show Execution Time
    (Rendering|Components|TextRender|SetText (Variables|Default|GetT_Time) (Utilities|Text|FormatText "{S} ms" (Utilities|Text|ToText(Float) (Class|KerasModel|GetLastExecuteTime (Variables|Default|GetKerasModel)) "HalfToEven" false true 1 1 5)))))

(fn ConstructionScript)

(fn BuildInputData
  (bind _handrightactor (Variables|Default|GetHandRightActor))
  (bind _handleftactor (Variables|Default|GetHandLeftActor))
  (bind _defaultsceneroot (Variables|/Game/Blueprints/BP_Hand.BP_Hand_C|GetDefaultSceneRoot _handrightactor))
  (bind _defaultsceneroot_2 (Variables|/Game/Blueprints/BP_Hand.BP_Hand_C|GetDefaultSceneRoot _handleftactor))
  (bind _returnvalue (Transformation|GetRelativeTransform _defaultsceneroot_2))
  (bind _returnvalue_2 (Transformation|GetRelativeTransform _defaultsceneroot))
  (return (Utilities|Array|MakeArray (.x (.location _returnvalue_2)) (.y (.location _returnvalue_2)) (.z (.location _returnvalue_2)) (.roll (.rotation _returnvalue_2)) (.pitch (.rotation _returnvalue_2)) (.yaw (.rotation _returnvalue_2)) (.x (.location _returnvalue)) (.y (.location _returnvalue)) (.z (.location _returnvalue)) (.roll (.rotation _returnvalue)) (.pitch (.rotation _returnvalue)) (.yaw (.rotation _returnvalue)))))

(fn UnpackOutput
  (params (InData :type Array%20of%20Floats%20%28double-precision%29))
  (bind _returnvalue (Transformation|GetActorTransform))
  (return (.location (Math|Transform|ComposeTransforms (Math|Conversions|ToTransform(Vector) (Math|Vector|MakeVector (Utilities|Array|Get(acopy) InData) (Utilities|Array|Get(acopy) InData 1) (Utilities|Array|Get(acopy) InData 2))) _returnvalue)) (.location (Math|Transform|ComposeTransforms (Math|Conversions|ToTransform(Vector) (Math|Vector|MakeVector (Utilities|Array|Get(acopy) InData 3) (Utilities|Array|Get(acopy) InData 4) (Utilities|Array|Get(acopy) InData 5))) _returnvalue))))